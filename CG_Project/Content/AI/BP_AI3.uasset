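; BP_AI3 is an AI character that fights in melee and takes damage until it dies.
; Damage lowers Health, either briefly halting movement with a hit montage or, at zero, ragdolling the mesh and destroying the actor after a delay.
; Attack, skipped when dead, plays a shove montage with a random chance of a sound.
; The montage's notify fires a forward sphere trace that damages the Pawn it hits.
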(event EventAttack
  (bind _returnvalue (Transformation|GetActorLocation))
  (if (not (Variables|Default|GetisDead))
    (Animation|Montage|PlayMontage (Variables|Character|GetMesh) "/Game/Characters/Mannequins/Animations/Paired_PushShove_Att_Montage.Paired_PushShove_Att_Montage"
      (:then
        (if (Math|Random|RandomBool)
          (Audio|PlaySoundatLocation "/Game/Audio/MS_AI_detect-sound.MS_AI_detect-sound" (Transformation|GetActorLocation) "0, 0, 0" 1.0 1.0 0.0 0 0 0 0)))
      (:OnNotifyBegin
        (bind (_outhit _returnvalue_2) (Collision|SphereTraceForObjects _returnvalue (+ _returnvalue (* (Math|Vector|GetForwardVector (Transformation|GetActorRotation)) 2e+02)) 3e+01 (Utilities|Array|MakeArray "ObjectTypeQuery3") false 0 "None"))
        (if _returnvalue_2
          (Game|Damage|ApplyDamage (.HitActor (Collision|BreakHitResult _outhit)) 1e+01 0 0))))))

(event Game|Damage|EventAnyDamage
  (params (Damage :type Float%20%28single-precision%29) (DamageType :type Damage%20Type%20Object%20Reference) (InstigatedBy :type Controller%20Object%20Reference) (DamageCauser :type Actor%20Object%20Reference))
  (Variables|Default|Sethealth (- (Variables|Default|Gethealth) Damage))
  (if (<= (Variables|Default|Gethealth) 0.0)
    (Physics|SetSimulatePhysics (Variables|Character|GetMesh) true)
    (Variables|Default|SetisDead true)
    (Pawn|Components|CharacterMovement|DisableMovement (Variables|Character|GetCharacterMovement))
    (Utilities|FlowControl|Delay 3.0)
    (Actor|DestroyActor)
    (else
      (Pawn|Components|CharacterMovement|DisableMovement (Variables|Character|GetCharacterMovement))
      (Animation|PlayAnimMontage "/Game/Characters/Mannequins/Animations/Manny/SK_Mannequin_Sequence_Montage_Hit_2.SK_Mannequin_Sequence_Montage_Hit_2" 1.0 "None")
      (Utilities|FlowControl|Delay 0.5)
      (Pawn|Components|CharacterMovement|SetMovementMode (Variables|Character|GetCharacterMovement) "MOVE_Walking" 0))))

(fn ConstructionScript)